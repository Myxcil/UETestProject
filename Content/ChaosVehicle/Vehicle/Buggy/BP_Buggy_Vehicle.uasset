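; BP_Buggy_Vehicle is a drivable Chaos buggy that passes player input to its vehicle movement component.
; BeginPlay adds the car's Enhanced Input mapping context to the possessing player controller.
; Throttle, steering, brake and handbrake actions share one setter for press and release, while gear up and down only set their shift inputs to true.
; Throttle input is also printed on screen for debugging.
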(event Input|EnhancedActionEvents|EnhancedInputActionIA_Throttle
  (params (ActionValue :type Float%20%28double-precision%29) (ElapsedSeconds :type Float%20%28double-precision%29) (TriggeredSeconds :type Float%20%28double-precision%29) (InputAction :type Input%20Action%20Object%20Reference :default "/Game/ChaosVehicle/Input/IA_Throttle.IA_Throttle"))
  (bind _vehiclemovementcomponent (Variables|Default|GetVehicleMovementComponent))
  (:Triggered
    (Class|ChaosVehicleMovementComponent|SetThrottleInput _vehiclemovementcomponent ActionValue :!label _label)
    (bind _returnvalue (Class|ChaosVehicleMovementComponent|GetThrottleInput _vehiclemovementcomponent))
    (Development|PrintString (Utilities|String|ToString(Float) _returnvalue)))
  (:Completed
    (goto _label)))

(event Input|EnhancedActionEvents|EnhancedInputActionIA_Brake
  (params (ActionValue :type Float%20%28double-precision%29) (ElapsedSeconds :type Float%20%28double-precision%29) (TriggeredSeconds :type Float%20%28double-precision%29) (InputAction :type Input%20Action%20Object%20Reference :default "/Game/ChaosVehicle/Input/IA_Brake.IA_Brake"))
  (:Triggered
    (Class|ChaosVehicleMovementComponent|SetBrakeInput (Variables|Default|GetVehicleMovementComponent) ActionValue :!label _label))
  (:Completed
    (goto _label)))

(event Input|EnhancedActionEvents|EnhancedInputActionIA_Handbrake
  (params (ActionValue :type Boolean) (ElapsedSeconds :type Float%20%28double-precision%29) (TriggeredSeconds :type Float%20%28double-precision%29) (InputAction :type Input%20Action%20Object%20Reference :default "/Game/ChaosVehicle/Input/IA_Handbrake.IA_Handbrake"))
  (:Started
    (Class|ChaosVehicleMovementComponent|SetHandbrakeInput (Variables|Default|GetVehicleMovementComponent) ActionValue :!label _label))
  (:Completed
    (goto _label)))

(event Input|EnhancedActionEvents|EnhancedInputActionIA_Steering
  (params (ActionValue :type Float%20%28double-precision%29) (ElapsedSeconds :type Float%20%28double-precision%29) (TriggeredSeconds :type Float%20%28double-precision%29) (InputAction :type Input%20Action%20Object%20Reference :default "/Game/ChaosVehicle/Input/IA_Steering.IA_Steering"))
  (:Triggered
    (Class|ChaosVehicleMovementComponent|SetSteeringInput (Variables|Default|GetVehicleMovementComponent) ActionValue :!label _label))
  (:Completed
    (goto _label)))

(event Input|EnhancedActionEvents|EnhancedInputActionIA_GearUp
  (params (ActionValue :type Boolean) (ElapsedSeconds :type Float%20%28double-precision%29) (TriggeredSeconds :type Float%20%28double-precision%29) (InputAction :type Input%20Action%20Object%20Reference :default "/Game/ChaosVehicle/Input/IA_GearUp.IA_GearUp"))
  (Class|ChaosVehicleMovementComponent|SetChangeUpInput (Variables|Default|GetVehicleMovementComponent) true))

(event Input|EnhancedActionEvents|EnhancedInputActionIA_GearDown
  (params (ActionValue :type Boolean) (ElapsedSeconds :type Float%20%28double-precision%29) (TriggeredSeconds :type Float%20%28double-precision%29) (InputAction :type Input%20Action%20Object%20Reference :default "/Game/ChaosVehicle/Input/IA_GearDown.IA_GearDown"))
  (Class|ChaosVehicleMovementComponent|SetChangeDownInput (Variables|Default|GetVehicleMovementComponent) true))

(event EventBeginPlay
  (bind _asplayer_controller (Utilities|Casting|CastToPlayerController (Pawn|GetController)))
  (Input|AddMappingContext (PlayerController|LocalPlayerSubsystems|GetEnhancedInputLocalPlayerSubsystem _asplayer_controller) "/Game/ChaosVehicle/Input/CarInputContext.CarInputContext" 0 "(bIgnoreAllPressedKeysUntilRelease=True,bForceImmediately=False,bNotifyUserSettings=False)"))

(fn ConstructionScript)